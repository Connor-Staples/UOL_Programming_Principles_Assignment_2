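; BP_SpaceLight is a light fixture that switches to red when its ButtonPress event fires.
; A reversed timeline drives greyscale colour and RectLight intensity, then a second timeline drives the red mesh colour and light intensity.
; ChangeColour writes the mesh materials' Colour parameter alongside the light changes.
; The construction script applies the Intensity variable to the RectLight in candelas.
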(event Custom|ButtonPress
  (bind _linear_track (Timeline|Timeline ReverseFromEnd)
    (:Update
      (CallFunction|ChangeColour (Math|Vector|MakeVector _linear_track _linear_track _linear_track))
      (Rendering|Components|Light|SetLightColor (Variables|Default|GetRectLight) (Math|Conversions|ToLinearColor(Vector) (Math|Vector|MakeVector _linear_track _linear_track _linear_track)) true)
      (Rendering|Components|Light|SetIntensity (Variables|Default|GetRectLight) (* _linear_track (Variables|Default|GetIntensity))))
    (:Finished
      (Rendering|Components|Light|SetLightColor (Variables|Default|GetRectLight) (Math|Conversions|ToLinearColor(Vector) (Math|Vector|MakeVector 255.0 0.0 0.0)) true)
      (bind _linear_track_2 (Timeline|Timeline_0 PlayFromStart)
        (:Update
          (CallFunction|ChangeColour (Math|Vector|MakeVector (* _linear_track_2 255.0) 0.0 0.0))
          (Rendering|Components|Light|SetIntensity (Variables|Default|GetRectLight) (* _linear_track_2 (Variables|Default|GetIntensity))))))))

(event EventBeginPlay)

(event Collision|EventActorBeginOverlap
  (params (OtherActor :type Actor%20Object%20Reference)))

(event EventTick
  (params (DeltaSeconds :type Float%20%28single-precision%29)))

(fn ConstructionScript
  (Rendering|Components|Light|SetIntensity (Variables|Default|GetRectLight) (Variables|Default|GetIntensity))
  (Class|LocalLightComponent|SetIntensityUnits (Variables|Default|GetRectLight) "Candelas"))

(fn ChangeColour
  (params (NewParam :type Vector))
  (Rendering|Material|SetVectorParameterValueonMaterials (Variables|Default|GetStaticMesh) "Colour" NewParam))