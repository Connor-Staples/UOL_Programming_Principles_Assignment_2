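; Root actor of an orbiter rotation puzzle, where buttons rotate orbiters around a sun sphere toward a target alignment.
; Button triggers, gated by a cooldown, add that button's per-orbiter angles to an integer rotation vector, then compare it, apparently modulo 360, to the target.
; On a match, chained timelines grow, then shrink and recolour the sun, before destroying the actors, setting player Cover and spawning teleporters inside the orbiter loop.
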(event Custom|Event%20ButtonTrigger
  (params (Button :type BP%20Button%20Object%20Reference))
  (bind _returnvalue (Transformation|GetActorTransform))
  (bind _returnvalue_2 (Math|Float|MakeLiteralFloat 0.01))
  (bind _buttons (Variables|Default|GetButtons))
  (bind _rotations (Variables|Default|GetRotations))
  (bind _returnvalue_3 (Utilities|Array|FindItem _buttons Button))
  (bind (_location _rotation _scale) (Math|Transform|BreakTransform _returnvalue))
  (bind _output (Utilities|Array|Get(acopy) _rotations _returnvalue_3))
  (bind (_x _y _z) (Utilities|Struct|BreakIntVector _output))
  (if (== (Variables|Default|GetButtonCooldown) 0.0)
    (bind _output_2 (CallFunction|IntVectorAdd _output (Variables|Default|GetRotationVec)))
    (for (_array_element _array_index) (Variables|Default|GetOrbiters)
      (Default|EventOrbit _array_element (Math|Conversions|ToFloat(Integer) (Utilities|Array|Get(acopy) (Utilities|Array|MakeArray _x _y _z) _array_index)) _array_element))
    (bind _output_get (Variables|Default|SetRotationVec _output_2))
    (bind _output_3 (CallFunction|IntVector% _output_get 360))
    (bind _output_4 (CallFunction|IntVectorEquality _output_3 (Variables|Default|GetTargetRotation)))
    (if _output_4
      (Development|PrintString "Puzzle Completed")
      (bind _sungrowtimeline (Timeline|Timeline_0 PlayFromStart)
        (:Update
          (Rendering|Material|SetScalarParameterValueonMaterials (Variables|Default|GetSphere) "Brightness" (+ (* _sungrowtimeline 0.5) 0.9))
          (Transformation|SetRelativeScale3D (Variables|Default|GetSphere) (* (Variables|Default|GetInitialScale) (+ (* _sungrowtimeline 0.5) 1.0))))
        (:Finished
          (Variables|Default|SetInitialScale (Variables|/Script/Engine.SceneComponent|GetRelativeScale3D (Variables|Default|GetSphere)))
          (bind _sun_shrink (Timeline|Timeline PlayFromStart)
            (:Update
              (Transformation|SetRelativeScale3D (Variables|Default|GetSphere) (* (Variables|Default|GetInitialScale) _sun_shrink))
              (if (<= _sun_shrink 0.4)
                (Rendering|Material|SetScalarParameterValueonMaterials (Variables|Default|GetSphere) "Brightness" (+ (* _sun_shrink 5.0) 1.4))
                (Rendering|Material|SetVectorParameterValueonMaterials (Variables|Default|GetSphere) "Colour 1" (+ (* (Math|Float|SafeDivide 1.0 _sun_shrink) (Math|Vector|MakeVector _returnvalue_2 _returnvalue_2 _returnvalue_2)) (Variables|Default|GetInitialColour1)))))
            (:Finished
              (Actor|DestroyActor)
              (Components|Activation|Activate (Variables|Default|GetEmitter) false)
              (for _array_element_2 (Variables|Default|GetOrbiters)
                (Actor|DestroyActor _array_element_2)
                (Variables|/Game/ThirdPerson/Blueprints/BP_ThirdPersonCharacter.BP_ThirdPersonCharacter_C|SetCover (Variables|Default|Getplayer) true)
                (Game|SpawnActorfromClass "/Game/MyBlueprints/BP_Teleporter.BP_Teleporter_C" (Math|Transform|MakeTransform _location "0, 0, 0" (* _scale "0.400000,0.400000,0.400000")) "Undefined" "MultiplyWithRoot" 0 0))))))
      (else
        (Development|PrintText (Utilities|Text|ToText(String) (Utilities|String|ToString(Integer) (Variables|Default|GetRotationVec))))))))

(event Collision|EventActorBeginOverlap
  (params (OtherActor :type Actor%20Object%20Reference))
  (|CallParentFunction OtherActor) ; This node is disabled and will not be called.\nDrag off pins to build functionality.
)

(event EventTick
  (params (DeltaSeconds :type Float%20%28single-precision%29))
  (|CallParentFunction DeltaSeconds)
  (if (> (Variables|Default|GetButtonCooldown) 0.0)
    (if (< (- (Variables|Default|GetButtonCooldown) DeltaSeconds) 0.0)
      (Variables|Default|SetButtonCooldown 0.0)
      (else
        (Variables|Default|SetButtonCooldown (- (Variables|Default|GetButtonCooldown) DeltaSeconds))))))

(event EventBeginPlay
  (bind _initialrotations (Variables|Default|GetInitialRotations))
  (bind _vector (CallFunction|VectortoIntVec (Math|Vector|MakeVector (Utilities|Array|Get(acopy) _initialrotations) (Utilities|Array|Get(acopy) _initialrotations 1) (Utilities|Array|Get(acopy) _initialrotations 2))))
  (Variables|Default|SetRotationVec _vector)
  (for (_array_element _array_index) (Variables|Default|GetOrbiters)
    (Default|Setup _array_element (Utilities|Array|Get(acopy) (Variables|Default|GetInitialRotations) _array_index) (Utilities|Array|Get(acopy) (Variables|Default|GetRadii) _array_index))
    (Variables|Default|SetButtonCooldown 0.0)
    (bind _asbp_third_person_character (Utilities|Casting|CastToBP_ThirdPersonCharacter (Game|Player|GetPlayerPawn 0)))
    (Variables|Default|Setplayer _asbp_third_person_character)
    (Variables|Default|SetInitialScale (Variables|/Script/Engine.SceneComponent|GetRelativeScale3D (Variables|Default|GetSphere)))
    (Variables|Default|SetInitialColour1 (* (Math|Vector|MakeVector 0.479167 0.218775 0.00769) (Math|Float|MakeLiteralFloat 255.0)))
    (Variables|Default|SetInitialColour2 (* (Math|Vector|MakeVector 1.0 0.871367 0.076185) (Math|Float|MakeLiteralFloat 255.0)))))

(fn ConstructionScript
  (|CallParentFunction))

(fn SunGrowAnimation)