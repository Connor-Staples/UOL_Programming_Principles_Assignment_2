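; Lockable door that raises while the player pawn is within its overlap area and lowers when they leave.
; ButtonPress, or starting unlocked, calls Unlock, which clears the lock and turns both indicator lights from red to green via material parameters.
; Tick moves the door incrementally, with a Seconds accumulator bounding travel and DoorOpenSpeed and DoorRaiseHeight setting the step.
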(event Custom|ButtonPress
  (CallFunction|Unlock))

(event EventBeginPlay
  (Variables|Default|SetPlayerInProximity false)
  (Variables|Default|SetSeconds 0.0)
  (if (not (Variables|Default|GetIsLocked))
    (CallFunction|Unlock)))

(event Collision|EventActorBeginOverlap
  (params (OtherActor :type Actor%20Object%20Reference))
  (if (== OtherActor (Game|Player|GetPlayerPawn 0))
    (Variables|Default|SetPlayerInProximity true)))

(event EventTick
  (params (DeltaSeconds :type Float%20%28single-precision%29))
  (bind _doorraiseheight (Variables|Default|GetDoorRaiseHeight))
  (bind _dooropenspeed (Variables|Default|GetDoorOpenSpeed))
  (bind _returnvalue (Math|Vector|MakeVector 0.0 0.0 _doorraiseheight))
  (bind _returnvalue_2 (Math|Float|SafeDivide DeltaSeconds _dooropenspeed))
  (bind _returnvalue_3 (* _returnvalue_2 _returnvalue))
  (if (== (Variables|Default|GetIsLocked) false)
    (if (Variables|Default|GetPlayerInProximity)
      (if (<= (Variables|Default|GetSeconds) (Variables|Default|GetDoorOpenSpeed))
        (Variables|Default|SetSeconds (+ (Variables|Default|GetSeconds) _returnvalue_2))
        (Transformation|SetWorldLocation (Variables|Default|GetDoor) (+ (Transformation|GetWorldLocation (Variables|Default|GetDoor)) _returnvalue_3) false false))
      (elif (>= (Variables|Default|GetSeconds) 0.0)
        (Variables|Default|SetSeconds (+ (* _returnvalue_2 -1.0) (Variables|Default|GetSeconds)))
        (Transformation|SetWorldLocation (Variables|Default|GetDoor) (+ (Math|Vector|NegateVector _returnvalue_3) (Transformation|GetWorldLocation (Variables|Default|GetDoor))) false false)))))

(event Collision|EventActorEndOverlap
  (params (OtherActor :type Actor%20Object%20Reference))
  (if (== OtherActor (Game|Player|GetPlayerPawn 0))
    (Variables|Default|SetPlayerInProximity false)))

(fn ConstructionScript
  (Rendering|Material|SetVectorParameterValueonMaterials (Variables|Default|GetLight) "Colour" "128.000000,0.000000,0.000000")
  (Rendering|Material|SetVectorParameterValueonMaterials (Variables|Default|GetLight1) "Colour" "128.000000,0.000000,0.000000"))

(fn Unlock
  (Variables|Default|SetIsLocked false)
  (Rendering|Material|SetVectorParameterValueonMaterials (Variables|Default|GetLight) "Colour" "0.000000,128.000000,0.000000")
  (Rendering|Material|SetVectorParameterValueonMaterials (Variables|Default|GetLight1) "Colour" "0.000000,128.000000,0.000000"))