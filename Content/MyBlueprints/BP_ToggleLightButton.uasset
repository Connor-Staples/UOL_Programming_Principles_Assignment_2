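; Floor-style button that, when the player pawn overlaps it, toggles the level's space lights and unlocks a linked door.
; BeginPlay caches every BP_SpaceLight; player overlap calls ButtonPress on each, with Door.Unlock inside the same loop.
; Any actor's overlap sets the pressed state, and any end overlap clears it.
; Tick uses that state and a timer to sink or raise the Cube and Plane along world Z.
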(event EventBeginPlay
  (Variables|Default|SetIsPressed false)
  (Variables|Default|SetSeconds 0.0)
  (bind _outactors (Actor|GetAllActorsOfClass "/Game/MyBlueprints/BP_SpaceLight.BP_SpaceLight_C"))
  (Variables|Default|SetLights _outactors))

(event Collision|EventActorBeginOverlap
  (params (OtherActor :type Actor%20Object%20Reference))
  (Variables|Default|SetIsPressed true)
  (if (== OtherActor (Game|Player|GetPlayerPawn 0))
    (for _array_element (Variables|Default|GetLights)
      (Default|ButtonPress _array_element)
      (Default|Unlock (Variables|Default|GetDoor)))))

(event EventTick
  (params (DeltaSeconds :type Float%20%28single-precision%29))
  (bind _fulldepthtime (Variables|Default|GetFullDepthTime))
  (bind _maxpressdepth (Variables|Default|GetMaxPressDepth))
  (bind _returnvalue (Math|Vector|MakeVector 0.0 0.0 _maxpressdepth))
  (bind _returnvalue_2 (Math|Float|SafeDivide 1.0 _fulldepthtime))
  (bind _returnvalue_3 (* DeltaSeconds _returnvalue_2))
  (bind _returnvalue_4 (* _returnvalue_3 _returnvalue))
  (bind _returnvalue_5 (Math|Vector|NegateVector _returnvalue_4))
  (if (Variables|Default|GetIsPressed)
    (if (<= (Variables|Default|GetSeconds) (Variables|Default|GetFullDepthTime))
      (Variables|Default|SetSeconds (+ (Variables|Default|GetSeconds) DeltaSeconds))
      (Transformation|SetWorldLocation (Variables|Default|GetCube) (+ _returnvalue_5 (Transformation|GetWorldLocation (Variables|Default|GetCube))) false false)
      (Transformation|SetWorldLocation (Variables|Default|GetPlane) (+ _returnvalue_5 (Transformation|GetWorldLocation (Variables|Default|GetPlane))) false false))
    (elif (>= (Variables|Default|GetSeconds) 0.0)
      (Variables|Default|SetSeconds (+ (* DeltaSeconds -1.0) (Variables|Default|GetSeconds)))
      (Transformation|SetWorldLocation (Variables|Default|GetCube) (+ _returnvalue_4 (Transformation|GetWorldLocation (Variables|Default|GetCube))) false false)
      (Transformation|SetWorldLocation (Variables|Default|GetPlane) (+ _returnvalue_4 (Transformation|GetWorldLocation (Variables|Default|GetPlane))) false false))))

(event Collision|EventActorEndOverlap
  (params (OtherActor :type Actor%20Object%20Reference))
  (Variables|Default|SetIsPressed false))

(fn ConstructionScript)