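; BP_Orbiter is an actor that circles a Pivot actor around the vertical axis in timed steps.
; Setup places it at a given radius and starting angle from the Pivot and resets its motion state.
; Orbit stores an angular distance and starts motion only when this instance is the named Orbiter.
; Tick rotates its offset from the Pivot over one second, trimming the final step to land on the requested angle.
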(event Custom|Event%20Orbit
  (params (Angular%20Distance :type Float%20%28double-precision%29) (Orbiter :type BP%20Orbiter%20Object%20Reference))
  (Variables|Default|SetAngular%20Distance Angular%20Distance)
  (if (== self Orbiter)
    (Variables|Default|SetRotate true)))

(event Custom|Setup
  (params (Initial%20Angle :type Float%20%28double-precision%29) (Radius :type Float%20%28double-precision%29))
  (Transformation|SetActorLocation (+ (Math|Vector|RotateVectorAroundAxis (Math|Vector|MakeVector 0.0 Radius 0.0) Initial%20Angle "0.000000,0.000000,1.000000") (Transformation|GetActorLocation (Variables|Default|GetPivot))) false false)
  (Variables|Default|SetElapsed%20TIme 0.0)
  (Variables|Default|SetRotate false)
  (Variables|Default|SetAngular%20Distance 0.0))

(event Custom|Set%20position)

(event EventBeginPlay)

(event Collision|EventActorBeginOverlap
  (params (OtherActor :type Actor%20Object%20Reference)))

(event EventTick
  (params (DeltaSeconds :type Float%20%28single-precision%29))
  (bind _returnvalue (Transformation|GetActorLocation))
  (bind _pivot (Variables|Default|GetPivot))
  (bind _returnvalue_2 (Transformation|GetActorLocation _pivot))
  (bind _returnvalue_3 (Math|Vector|NegateVector _returnvalue_2))
  (bind _returnvalue_4 (+ _returnvalue_3 _returnvalue))
  (if (Variables|Default|GetRotate)
    (if (>= (+ (Variables|Default|GetElapsed%20TIme) DeltaSeconds) (Math|Float|MakeLiteralFloat 1.0))
      (Transformation|SetActorLocation (+ (Math|Vector|RotateVectorAroundAxis _returnvalue_4 (* (- (Math|Float|MakeLiteralFloat 1.0) (Variables|Default|GetElapsed%20TIme)) (Variables|Default|GetAngular%20Distance)) "0.000000,0.000000,1.000000") (Transformation|GetActorLocation (Variables|Default|GetPivot))) false false)
      (Variables|Default|SetRotate false)
      (Variables|Default|SetElapsed%20TIme 0.0)
      (else
        (Transformation|SetActorLocation (+ (Math|Vector|RotateVectorAroundAxis _returnvalue_4 (* (Variables|Default|GetAngular%20Distance) DeltaSeconds) "0.000000,0.000000,1.000000") _returnvalue_2) false false)
        (Variables|Default|SetElapsed%20TIme (+ (Variables|Default|GetElapsed%20TIme) DeltaSeconds))))))

(fn ConstructionScript)